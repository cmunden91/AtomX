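; Bit panel actor that lights up when the player's collected bit count matches the number stored in its root component's tag.
; Each tick it loops over all ThirdPersonCharacter actors and its tags with empty loop bodies, then compares the final tag, converted to an integer, to the final character's BitsCollected.
; On an exact match it swaps the plane's material and unhides the point light, with no revert logic.
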(event EventBeginPlay)

(event Collision|EventActorBeginOverlap
  (params (OtherActor :type Actor%20Object%20Reference)))

(event EventTick
  (params (DeltaSeconds :type Float%20%28single-precision%29))
  (bind _outactors (Actor|GetAllActorsOfClass "/Game/AtomX/BluePrints/ThirdPersonCharacter.ThirdPersonCharacter_C"))
  (for _array_element _outactors
    _)
  (for _array_element_2 (Variables|/Script/Engine.ActorComponent|GetComponentTags (Variables|Default|GetDefaultSceneRoot))
    _)
  (if (== (Math|Conversions|ToInteger(Byte) (Utilities|String|ToString(Name) _array_element_2)) (Variables|/Game/AtomX/BluePrints/ThirdPersonCharacter.ThirdPersonCharacter_C|GetBitsCollected _array_element))
    (Rendering|Material|SetMaterial (Variables|Default|GetPlane1) 0 "/Game/AtomX/Textures/QuantumBitPic_-_Copy_Mat_2.QuantumBitPic_-_Copy_Mat_2")
    (Development|SetHiddeninGame (Variables|Default|GetPointLight) false false)))

(fn ConstructionScript)